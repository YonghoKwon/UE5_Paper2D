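; Paper2D knight Blueprint that drives four-direction idle, move and attack sprite animation from player input.
; Each tick, UpdateInput derives facing and a moving flag from the axes, with horizontal overriding vertical, then UpdateAnimation selects the flipbook.
; The Attack action sets a flag that takes priority over idle and move for the flipbook's length.
; Left and right share side flipbooks, mirrored by rotating the sprite.
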(event EventTick
  (params (DeltaSeconds :type Float%20%28single-precision%29))
  (CallFunction|UpdateInput)
  (CallFunction|UpdateAnimation))

(event Input|ActionEvents|InputActionAttack
  (params (Key :type Key%20Structure :default "None"))
  (:Pressed
    (Variables|Default|SetbAttack true)
    (CallFunction|UpdateAnimation)
    (Utilities|FlowControl|Delay (Class|PaperFlipbookComponent|GetFlipbookLength (Variables|Default|GetSprite)))
    (Variables|Default|SetbAttack false)))

(fn ConstructionScript)

(fn UpdateAnimation
  (bind _sprite (Variables|Default|GetSprite))
  (bind _sprite_2 (Variables|Default|GetSprite))
  (bind _sprite_3 (Variables|Default|GetSprite))
  (if (Variables|Default|GetbAttack)
    (switch Utilities|FlowControl|Switch|SwitchonEDirection (Variables|Default|GetDirection)
      (:NewEnumerator0
        (Sprite|SetFlipbook _sprite_2 "/Game/Sprites/Knight/up_attack.up_attack"))
      (:NewEnumerator1
        (Sprite|SetFlipbook _sprite_2 "/Game/Sprites/Knight/down_attack.down_attack"))
      (:NewEnumerator2
        (Sprite|SetFlipbook _sprite_2 "/Game/Sprites/Knight/side_attack.side_attack")
        (Transformation|SetRelativeRotation _sprite_2 "0,180.000000, 0" false false))
      (:NewEnumerator3
        (Sprite|SetFlipbook _sprite_2 "/Game/Sprites/Knight/side_attack.side_attack")
        (Transformation|SetRelativeRotation _sprite_2 "0, 0, 0" false false)))
    (elif (not (Variables|Default|GetbKeyboardPressed))
      (switch Utilities|FlowControl|Switch|SwitchonEDirection (Variables|Default|GetDirection)
        (:NewEnumerator0
          (Sprite|SetFlipbook _sprite_3 "/Game/Sprites/Knight/up_idle.up_idle"))
        (:NewEnumerator1
          (Sprite|SetFlipbook _sprite_3 "/Game/Sprites/Knight/down_idle.down_idle"))
        (:NewEnumerator2
          (Sprite|SetFlipbook _sprite_3 "/Game/Sprites/Knight/side_idle.side_idle")
          (Transformation|SetRelativeRotation _sprite_3 "0,180.000000, 0" false false))
        (:NewEnumerator3
          (Sprite|SetFlipbook _sprite_3 "/Game/Sprites/Knight/side_idle.side_idle")
          (Transformation|SetRelativeRotation _sprite_3 "0,0.000000, 0" false false)))
      (else
        (switch Utilities|FlowControl|Switch|SwitchonEDirection (Variables|Default|GetDirection)
          (:NewEnumerator0
            (Sprite|SetFlipbook _sprite "/Game/Sprites/Knight/up_move.up_move"))
          (:NewEnumerator1
            (Sprite|SetFlipbook _sprite "/Game/Sprites/Knight/down_move.down_move"))
          (:NewEnumerator2
            (Sprite|SetFlipbook _sprite "/Game/Sprites/Knight/side_move.side_move")
            (Transformation|SetRelativeRotation _sprite "0,180.000000, 0" false false))
          (:NewEnumerator3
            (Sprite|SetFlipbook _sprite "/Game/Sprites/Knight/side_move.side_move")
            (Transformation|SetRelativeRotation _sprite "0, 0, 0" false false)))))))

(fn UpdateInput
  (Utilities|FlowControl|Sequence
    (:then_0
      (Variables|Default|SetbKeyboardPressed (or (!= (Input|AxisValues|GetMoveUp) 0.0) (!= (Input|AxisValues|GetMoveRight) 0.0))))
    (:then_1
      (Math|Float|CompareFloat (Input|AxisValues|GetMoveUp) 0.0
        (:>
          (Variables|Default|SetDirection "NewEnumerator0"))
        (:<
          (Variables|Default|SetDirection "NewEnumerator1"))))
    (:then_2
      (Math|Float|CompareFloat (Input|AxisValues|GetMoveRight) 0.0
        (:>
          (Variables|Default|SetDirection "NewEnumerator3"))
        (:<
          (Variables|Default|SetDirection "NewEnumerator2"))))))